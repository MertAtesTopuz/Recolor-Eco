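; Quest manager that steps through an ordered array of quest actors, one active quest at a time.
; On BeginPlay it registers itself on Yunus_GI_GameInstance and starts the first progression.
; Each ProgressQuest call deactivates the previous actor, activates the current one through quest messages, then increments the index.
; SetQuestActive is an empty stub.
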(event EventBeginPlay
  (bind _asyunus_gi_game_instance (Utilities|Casting|CastToYunus_GI_GameInstance (Game|GetGameInstance)))
  (Variables|/Game/DevelopmentMain/YunusMain/Blueprints/Player/Yunus_GI_GameInstance.Yunus_GI_GameInstance_C|SetQuestManager _asyunus_gi_game_instance self)
  (CallFunction|ProgressQuest))

(event EventProgressQuest
  (bind _questactors (Variables|Default|GetQuestActors))
  (bind _questindex (Variables|Default|GetQuestIndex))
  (bind _questactors_2 (Variables|Default|GetQuestActors))
  (bind _questindex_2 (Variables|Default|GetQuestIndex))
  (bind _output (Utilities|Array|Get(acopy) _questactors _questindex))
  (bind _returnvalue (- _questindex_2 1))
  (bind _output_2 (Utilities|Array|Get(acopy) _questactors_2 _returnvalue))
  (Utilities|IsValid _output_2
    (:Is%20Valid
      (Class|YunusBPIQuesterFace|DeactiveQuest(Message) _output_2))
    (:Is%20Not%20Valid
      _))
  (Utilities|IsValid _output
    (:Is%20Valid
      (Class|YunusBPIQuesterFace|ActiveQuest(Message) _output))
    (:Is%20Not%20Valid
      _))
  (Math|Integer|IncrementInt (Variables|Default|GetQuestIndex)))

(fn ConstructionScript)

(fn SetQuestActive)