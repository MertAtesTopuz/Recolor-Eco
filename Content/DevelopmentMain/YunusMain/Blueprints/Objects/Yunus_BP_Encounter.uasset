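; An interactable encounter actor that shows a "press E" prompt when the player enters its sphere and opens an encounter status panel.
; The Encounterface event, gated on prompt visibility, blends the view to this actor, disables character input and reveals the EncounterStatus widget.
; On BeginPlay that widget receives a self reference and the level name.
; CloseEncounter restores the player's view, input and prompt.
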(event OnComponentBeginOverlap(Sphere)
  (params (OverlappedComponent :type Primitive%20Component%20Object%20Reference) (OtherActor :type Actor%20Object%20Reference) (OtherComp :type Primitive%20Component%20Object%20Reference) (OtherBodyIndex :type Integer) (bFromSweep :type Boolean) (SweepResult :type Hit%20Result%20Structure%20%28by%20ref%29))
  (if (Actor|ActorHasTag OtherActor "Player")
    (Rendering|SetVisibility (Variables|Default|GetPressE) true false)))

(event OnComponentEndOverlap(Sphere)
  (params (OverlappedComponent :type Primitive%20Component%20Object%20Reference) (OtherActor :type Actor%20Object%20Reference) (OtherComp :type Primitive%20Component%20Object%20Reference) (OtherBodyIndex :type Integer))
  (if (Actor|ActorHasTag OtherActor "Player")
    (Rendering|SetVisibility (Variables|Default|GetPressE) false false)))

(event EventEncounterface
  (if (Variables|/Script/Engine.SceneComponent|GetbVisible (Variables|Default|GetPressE))
    (Game|Player|SetViewTargetwithBlend (Game|GetPlayerController 0) self 0.5 "VTBlend_Linear" 0.0 false)
    (Input|DisableInput (Game|GetPlayerCharacter 0) (Game|GetPlayerController 0))
    (Rendering|SetVisibility (Variables|Default|GetPressE) false false)
    (Rendering|SetVisibility (Variables|Default|GetEncounterStatus) true false)))

(event EventBeginPlay
  (bind _asyunus_wbp_encounter_status (Utilities|Casting|CastToYunus_WBP_EncounterStatus (UserInterface|GetWidget (Variables|Default|GetEncounterStatus))))
  (Variables|/Game/DevelopmentMain/YunusMain/Blueprints/UI/InGameUI/Yunus_WBP_EncounterStatus.Yunus_WBP_EncounterStatus_C|SetEncounter _asyunus_wbp_encounter_status self)
  (Variables|/Game/DevelopmentMain/YunusMain/Blueprints/UI/InGameUI/Yunus_WBP_EncounterStatus.Yunus_WBP_EncounterStatus_C|SetLevel%20Name _asyunus_wbp_encounter_status (Variables|Default|GetLevel%20Name)))

(fn ConstructionScript)

(fn CloseEncounter
  (Game|Player|SetViewTargetwithBlend (Game|GetPlayerController 0) (Game|GetPlayerCharacter 0) 0.5 "VTBlend_Linear" 0.0 false)
  (Rendering|SetVisibility (Variables|Default|GetEncounterStatus) false false)
  (Input|EnableInput (Game|GetPlayerController 0) 0)
  (Rendering|SetVisibility (Variables|Default|GetPressE) true false))