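; Van manager actor that sets up the van scene when its level begins.
; On BeginPlay it caches the game instance, binds to its BeginLevel event and deactivates the player.
; When the level begins, it registers itself with the current Van UI widget and switches the player's view to the first camera in its Cameras array.
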(event Custom|BeginLevel_Event
  (bind _asyunus_wbp_van_ui (Utilities|Casting|CastToYunus_WBP_VanUI (Variables|/Game/DevelopmentMain/YunusMain/Blueprints/Player/Yunus_GI_GameInstance.Yunus_GI_GameInstance_C|GetCurrentUI (stale EventBeginPlay _output_get))))
  (Variables|/Game/DevelopmentMain/YunusMain/Blueprints/UI/Yunus_WBP_VanUI.Yunus_WBP_VanUI_C|SetVanManager _asyunus_wbp_van_ui self)
  (Game|Player|SetViewTargetwithBlend (Game|GetPlayerController 0) (Utilities|Array|Get(acopy) (Variables|Default|GetCameras)) 0.0 "VTBlend_Linear" 0.0 false))

(event EventBeginPlay
  (bind _asyunus_gi_game_instance (Utilities|Casting|CastToYunus_GI_GameInstance (Game|GetGameInstance)))
  (bind _output_get (Variables|Default|SetGameInstance _asyunus_gi_game_instance))
  (EventDispatchers|AssignBeginLevel _output_get (delegate Custom|BeginLevel_Event))
  (Default|SetPlayerActive _output_get false))

(fn ConstructionScript)