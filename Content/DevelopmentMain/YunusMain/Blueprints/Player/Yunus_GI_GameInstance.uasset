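; Game instance that manages game state, streamed level transitions, UI and background music.
; Load and unload events map a song enum to a streamed level behind an animated loading screen, then set the new state.
; CreateUI swaps the active widget by state; loading also fades music, with a track set only for Van.
; Helpers toggle player visibility, movement and camera target, and bank player points into a running total.
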(event Custom|LoadLevel
  (params (Level :type Yunus_E_LevelName%20Enum :default "NewEnumerator0") (State :type Yunus_E_GameState%20Enum :default "NewEnumerator6"))
  ;[0.15 0.15 0.15 0.5] Level loader
  (Variables|Game|SetGameState "NewEnumerator1")
  (bind _returnvalue (UserInterface|CreateWidget "/Game/DevelopmentMain/YunusMain/Blueprints/UI/MainUIs/Yunus_WBP_LoadingScreen.Yunus_WBP_LoadingScreen_C" 0 self))
  (UserInterface|Viewport|AddtoViewport _returnvalue 999)
  (bind _backgroundmusic (Variables|Default|GetBackgroundMusic)
    (:then
      (Audio|Components|Audio|FadeOut _backgroundmusic 0.5 0.0 "Linear" :!class /Script/Engine.AudioComponent))
    (:else
      _))
  (UserInterface|Animation|PlayAnimation _returnvalue (Variables|/Game/DevelopmentMain/YunusMain/Blueprints/UI/MainUIs/Yunus_WBP_LoadingScreen.Yunus_WBP_LoadingScreen_C|GetLoadingScreen _returnvalue) 0.0 1 "Forward" 1.0 false)
  (Utilities|FlowControl|Delay (Variables|Other|GetExtraTime))
  (Class|GameplayStatics|LoadStreamLevelbySoftObjectPtr (CallFunction|SongtoWorld Level) true false)
  (UserInterface|Animation|PlayAnimation _returnvalue (Variables|/Game/DevelopmentMain/YunusMain/Blueprints/UI/MainUIs/Yunus_WBP_LoadingScreen.Yunus_WBP_LoadingScreen_C|GetClearLoadingScreen _returnvalue) 0.0 1 "Forward" 1.0 false)
  (Variables|Game|SetGameState State)
  (CallFunction|CreateUI)
  (bind _returnvalue_2 (Audio|SpawnSound2D (Utilities|Select :Index (Variables|Game|GetGameState) :NewEnumerator6 0 :NewEnumerator0 0 :NewEnumerator1 0 :NewEnumerator2 0 :NewEnumerator3 0 :NewEnumerator4 0 :NewEnumerator5 0 :NewEnumerator7 "/Game/DevelopmentMain/YunusMain/Assets/Audio/Yunus_SW_VanOpen.Yunus_SW_VanOpen") 1.0 1.0 0.0 0))
  (Utilities|IsValid _returnvalue_2
    (:Is%20Valid
      (Audio|Components|Audio|FadeIn _returnvalue_2 0.5 1.0 0.0 "Linear" :!class /Script/Engine.AudioComponent)
      (Variables|Default|SetBackgroundMusic _returnvalue_2))
    (:Is%20Not%20Valid
      _))
  (Default|CallBeginLevel))

(event Custom|UnloadLevel
  (params (Level :type Yunus_E_LevelName%20Enum :default "NewEnumerator0"))
  ;[0.15 0.15 0.15 0.5] Level unloader
  (Variables|Game|SetGameState "NewEnumerator1")
  (bind _returnvalue (UserInterface|CreateWidget "/Game/DevelopmentMain/YunusMain/Blueprints/UI/MainUIs/Yunus_WBP_LoadingScreen.Yunus_WBP_LoadingScreen_C" 0 self))
  (UserInterface|Viewport|AddtoViewport _returnvalue 999)
  (UserInterface|Animation|PlayAnimation _returnvalue (Variables|/Game/DevelopmentMain/YunusMain/Blueprints/UI/MainUIs/Yunus_WBP_LoadingScreen.Yunus_WBP_LoadingScreen_C|GetLoadingScreen _returnvalue) 0.0 1 "Forward" 1.0 false)
  (Utilities|FlowControl|Delay (Variables|Other|GetExtraTime))
  (Class|GameplayStatics|UnloadStreamLevelbySoftObjectPtr (CallFunction|SongtoWorld Level) false)
  (CallFunction|SetPlayerActive true)
  (UserInterface|Animation|PlayAnimation _returnvalue (Variables|/Game/DevelopmentMain/YunusMain/Blueprints/UI/MainUIs/Yunus_WBP_LoadingScreen.Yunus_WBP_LoadingScreen_C|GetClearLoadingScreen _returnvalue) 0.0 1 "Forward" 1.0 false)
  (Variables|Game|SetGameState "NewEnumerator2")
  (CallFunction|CreateUI))

(fn CreateUI
  (Utilities|IsValid (Variables|Game|GetCurrentUI)
    (:Is%20Valid
      (Widget|RemovefromParent (Variables|Game|GetCurrentUI)))
    (:Is%20Not%20Valid
      _))
  (bind _returnvalue (UserInterface|CreateWidget (Utilities|Select :Index (Variables|Game|GetGameState) :NewEnumerator6 0 :NewEnumerator0 "/Game/DevelopmentMain/YunusMain/Blueprints/UI/MainUIs/Yunus_WB_StartMenu.Yunus_WB_StartMenu_C" :NewEnumerator1 0 :NewEnumerator2 "/Game/DevelopmentMain/YunusMain/Blueprints/UI/MainUIs/Yunus_WB_PlayerMainUI.Yunus_WB_PlayerMainUI_C" :NewEnumerator3 "/Game/DevelopmentMain/YunusMain/Blueprints/UI/MainUIs/Yunus_WB_PlayerGameUI.Yunus_WB_PlayerGameUI_C" :NewEnumerator4 0 :NewEnumerator5 0 :NewEnumerator7 "/Game/DevelopmentMain/YunusMain/Blueprints/UI/UpgradeUI/Yunus_WBP_VanUI.Yunus_WBP_VanUI_C")))
  (bind _output_get (Variables|Game|SetCurrentUI _returnvalue))
  (UserInterface|Viewport|AddtoViewport _output_get 0))

(fn SongtoWorld
  (params (Song :type Yunus_E_LevelName%20Enum :default "NewEnumerator0"))
  (return (Utilities|Select :Index Song :NewEnumerator2 (LocalVariables|GetL-City) :NewEnumerator0 (LocalVariables|GetL-PartyToNight) :NewEnumerator3 (LocalVariables|GetL-Van) :NewEnumerator1 0 :NewEnumerator4 (LocalVariables|GetL-Final))))

(fn SetPlayerActive
  (params (Active :type Boolean))
  (bind _player (Variables|Game|GetPlayer))
  (Rendering|SetVisibility (Variables|/Script/Engine.Character|GetMesh _player) Active false)
  (Variables|/Game/DevelopmentMain/YunusMain/Blueprints/Player/Yunus_BP_ThirdPersonCharacter.Yunus_BP_ThirdPersonCharacter_C|SetCanMove _player Active)
  (if Active
    (Game|Player|SetViewTargetwithBlend (Game|GetPlayerController 0) (Variables|Game|GetPlayer) 0.0 "VTBlend_Linear" 0.0 false)))

(fn CalculatePoints
  (bind _player (Variables|Game|GetPlayer))
  (Variables|Currency|SetTotalPoints (+ (Variables|/Game/DevelopmentMain/YunusMain/Blueprints/Player/Yunus_BP_ThirdPersonCharacter.Yunus_BP_ThirdPersonCharacter_C|GetPoints _player) (Variables|Currency|GetTotalPoints)))
  (Variables|/Game/DevelopmentMain/YunusMain/Blueprints/Player/Yunus_BP_ThirdPersonCharacter.Yunus_BP_ThirdPersonCharacter_C|SetPoints _player 0))