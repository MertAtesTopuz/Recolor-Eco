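; Game mode for an encounter level that sets up the player and awards points when the encounter ends.
; On BeginPlay it starts the player character's game, disables its movement, switches to the game camera and caches the game instance.
; ReturnToMainHub converts sufficiently high gained points into ColorPoint on the game instance.
; Despite its name it does not change level, as the ChangeLevel call is unconnected.
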(event Custom|ReturnToMainHub
  (params (GainedPoints :type Integer))
  (bind _as_yunus_gi_game_instance (Variables|Default|GetAs%20Yunus%20GI%20Game%20Instance))
  (Utilities|FlowControl|Sequence
    (:then_0
      (if (>= GainedPoints 30)
        (Variables|/Game/DevelopmentMain/YunusMain/Blueprints/Player/Yunus_GI_GameInstance.Yunus_GI_GameInstance_C|SetColorPoint _as_yunus_gi_game_instance (+ (/ GainedPoints 20) (Variables|/Game/DevelopmentMain/YunusMain/Blueprints/Player/Yunus_GI_GameInstance.Yunus_GI_GameInstance_C|GetColorPoint _as_yunus_gi_game_instance)))))
    (:then_1)))

(event EventBeginPlay
  (Utilities|FlowControl|Sequence
    (:then_0
      (bind _asyunus_bp_third_person_character (Utilities|Casting|CastToYunus_BP_ThirdPersonCharacter (Game|GetPlayerCharacter 0)))
      (bind _output_get (Variables|Default|SetPlayer _asyunus_bp_third_person_character))
      (Default|LettheGamesBegin _output_get)
      (Variables|/Game/DevelopmentMain/YunusMain/Blueprints/Player/Yunus_BP_ThirdPersonCharacter.Yunus_BP_ThirdPersonCharacter_C|SetCanMove _output_get false)
      (Default|SetGameCamera _output_get)
      (bind _asyunus_gi_game_instance (Utilities|Casting|CastToYunus_GI_GameInstance (Game|GetGameInstance)))
      (Variables|Default|SetAs%20Yunus%20GI%20Game%20Instance _asyunus_gi_game_instance))
    (:then_1
      (Development|PrintString "1"))))

(fn ConstructionScript)