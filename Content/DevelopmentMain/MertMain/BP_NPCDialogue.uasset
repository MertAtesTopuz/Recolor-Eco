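; BP_NPCDialogue is an NPC that shows a press-E prompt in its trigger zone while its quest is active or its mission is finished.
; Each interact steps through one of three dialogue arrays (first talk, repeat, mission finished), updating a UI widget with text, name, portrait and sound.
; After the last line it closes the widget and shows the quest text on the player's mission UI.
; QuestManager is cached, but its ProgressQuest call is unwired.
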(event OnComponentBeginOverlap(TriggerZone)
  (params (OverlappedComponent :type Primitive%20Component%20Object%20Reference) (OtherActor :type Actor%20Object%20Reference) (OtherComp :type Primitive%20Component%20Object%20Reference) (OtherBodyIndex :type Integer) (bFromSweep :type Boolean) (SweepResult :type Hit%20Result%20Structure%20%28by%20ref%29))
  (if (Actor|ActorHasTag OtherActor "Player")
    (if (Variables|Bools|GetIsMissionFinished)
      (Rendering|SetVisibility (Variables|Default|GetPressE) true false :!label _label)
      (elif (Variables|Bools|GetcanQuest)
        (goto _label)))))

(event OnComponentEndOverlap(TriggerZone)
  (params (OverlappedComponent :type Primitive%20Component%20Object%20Reference) (OtherActor :type Actor%20Object%20Reference) (OtherComp :type Primitive%20Component%20Object%20Reference) (OtherBodyIndex :type Integer))
  (if (Actor|ActorHasTag OtherActor "Player")
    (Rendering|SetVisibility (Variables|Default|GetPressE) false false)))

(event EventBeginPlay
  (bind _asyunus_gi_game_instance (Utilities|Casting|CastToYunus_GI_GameInstance (Game|GetGameInstance)))
  (Variables|Quest|SetQuest%20Manager (Variables|/Game/DevelopmentMain/YunusMain/Blueprints/Player/Yunus_GI_GameInstance.Yunus_GI_GameInstance_C|GetQuestManager _asyunus_gi_game_instance))
  (bind _asyunus_bp_third_person_character (Utilities|Casting|CastToYunus_BP_ThirdPersonCharacter (Game|GetPlayerCharacter 0)))
  (Variables|Default|SetAs%20Yunus%20BP%20Third%20Person%20Character _asyunus_bp_third_person_character))

(event EventActiveQuest
  (Variables|Bools|SetcanQuest true))

(event EventDeactiveQuest
  (Variables|Bools|SetcanQuest false))

(event EventInterractface
  (if (Variables|Bools|GetIsMissionFinished)
    (Rendering|SetVisibility (Variables|Default|GetPressE) false false :!label _label)
    (CallFunction|DialogueFunction (Utilities|Select :Index (Variables|Dialogues|GetNewVar) :NewEnumerator0 (Variables|Dialogues|GetDialogue) :NewEnumerator1 (Variables|Dialogues|GetSecondDialogue) :NewEnumerator2 (Variables|Dialogues|GetFinishedMissionDialogue) :NewEnumerator3 0))
    (if (Variables|Bools|GetIsFirstTalk)
      (if (Variables|Bools|GetIsMissionFinished)
        (Variables|Dialogues|SetNewVar "NewEnumerator2")
        (else
          (Variables|Dialogues|SetNewVar "NewEnumerator1")))
      (else
        (Variables|Dialogues|SetNewVar "NewEnumerator0")))
    (elif (Variables|Bools|GetcanQuest)
      (goto _label))))

(fn ConstructionScript)

(fn DialogueFunction
  (params (DialogueType :type Array%20of%20Strings))
  (Math|Integer|IncrementInt (Variables|Default|GetTalkIndex)
    (:%20%20
      (if (< (Variables|Default|GetTalkIndex) (Utilities|Array|Length DialogueType))
        (Variables|Default|GetDialogueUI
          (:then
            _)
          (:else
            (bind _returnvalue (UserInterface|CreateWidget "/Game/DevelopmentMain/MertMain/Mert_WB_DialogueUI.Mert_WB_DialogueUI_C" (Game|GetPlayerController 0)))
            (bind _output_get (Variables|Default|SetDialogueUI _returnvalue))
            (UserInterface|Viewport|AddtoViewport _output_get 0)))
        (Rendering|Components|TextRender|SetText (Variables|/Game/DevelopmentMain/MertMain/Mert_WB_DialogueUI.Mert_WB_DialogueUI_C|GetTalkText (Variables|Default|GetDialogueUI)) (Utilities|Text|ToText(String) (Utilities|Array|Get(acopy) DialogueType (Variables|Default|GetTalkIndex))))
        (CallFunction|SetCharacterApperience)
        (Audio|PlaySound2D (Variables|ChaIdentity|GetNPCSound) 1.0 1.0 0.0 0 0)
        (else
          (Variables|Bools|SetIsFirstTalk true)
          (Variables|Default|SetTalkIndex -1)
          (Widget|RemovefromParent (Variables|Default|GetDialogueUI))
          (Variables|Default|SetDialogueUI 0)
          (Rendering|SetVisibility (Variables|Default|GetPressE) true false)
          (CallFunction|SetMissionDialogue))))))

(fn SetCharacterApperience
  (Rendering|Components|TextRender|SetText (Variables|/Game/DevelopmentMain/MertMain/Mert_WB_DialogueUI.Mert_WB_DialogueUI_C|GetNameText (Variables|Default|GetDialogueUI)) (Utilities|Array|Get(acopy) (Variables|ChaIdentity|GetCharacterName) (Variables|Default|GetTalkIndex)))
  (Appearance|SetBrushfromTexture (Variables|/Game/DevelopmentMain/MertMain/Mert_WB_DialogueUI.Mert_WB_DialogueUI_C|GetCharacterImage (Variables|Default|GetDialogueUI)) (Variables|ChaIdentity|GetCharacterImage) false))

(fn NewFunction
  (params (NewVar :type Mert_E_DialogueTypes%20Enum :default "NewEnumerator0"))
  (Variables|Dialogues|SetNewVar NewVar))

(fn SetMissionDialogue
  (bind _as_yunus_bp_third_person_character (Variables|Default|GetAs%20Yunus%20BP%20Third%20Person%20Character))
  (bind _missionui (Variables|/Game/DevelopmentMain/YunusMain/Blueprints/Player/Yunus_BP_ThirdPersonCharacter.Yunus_BP_ThirdPersonCharacter_C|GetMissionUI _as_yunus_bp_third_person_character))
  (bind _missiontxt (Variables|/Game/DevelopmentMain/MertMain/Mert_WB_MissionUI.Mert_WB_MissionUI_C|GetMissionTxt _missionui))
  (Widget|SetVisibility _missiontxt "Visible")
  (Rendering|Components|TextRender|SetText _missiontxt (Variables|Quest|GetQuestText)))